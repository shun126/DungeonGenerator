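; BP_TopView_DungeonDoor is a top-view dungeon door whose shutter moves vertically as the player passes through its trigger.
; Box overlap by player pawn 0 plays the ShutterOpen timeline from the start, and leaving the box reverses it.
; The timeline's Offset track sets the static mesh's relative Z location, teleporting without sweep.
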(event `self.Box.OnComponentBeginOverlap`
  (params (OverlappedComponent :type "PrimitiveComponent Object Reference") (OtherActor :type "Actor Object Reference") (OtherComp :type "PrimitiveComponent Object Reference") (OtherBodyIndex :type Integer) (bFromSweep :type Boolean) (SweepResult :type "HitResult Structure (by ref)"))
  (if (== OtherActor (`GameplayStatics.GetPlayerPawn` 0))
    (`TimelineComponent.PlayFromStart` (`self.ShutterOpen`))))

(event `self.Box.OnComponentEndOverlap`
  (params (OverlappedComponent :type "PrimitiveComponent Object Reference") (OtherActor :type "Actor Object Reference") (OtherComp :type "PrimitiveComponent Object Reference") (OtherBodyIndex :type Integer))
  (if (== OtherActor (`GameplayStatics.GetPlayerPawn` 0))
    (`TimelineComponent.Reverse` (`self.ShutterOpen`))))

(fn `UserConstructionScript`)