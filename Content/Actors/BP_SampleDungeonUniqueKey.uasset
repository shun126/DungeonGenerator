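; BP_SampleDungeonUniqueKey is a sample dungeon pickup actor for a unique key, with a spinning text render.
; Tick adds yaw to the text each frame from a delta-time-scaled rate plus the TextRotation variable, which is not time-scaled.
; Overlap of the sphere by the first player's pawn prints a placeholder message and destroys the actor.
; Adding the key to inventory is not implemented.
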(event `self.ReceiveTick`
  (params (DeltaSeconds :type "Float (single-precision)"))
  (`SceneComponent.K2_AddLocalRotation` (`self.TextRender`) (`KismetMathLibrary.MakeRotator` 0.0 0.0 (+ (* DeltaSeconds 90.0) (`self.TextRotation`))) false false))

(event `self.Sphere.OnComponentBeginOverlap`
  (params (OverlappedComponent :type "PrimitiveComponent Object Reference") (OtherActor :type "Actor Object Reference") (OtherComp :type "PrimitiveComponent Object Reference") (OtherBodyIndex :type Integer) (bFromSweep :type Boolean) (SweepResult :type "HitResult Structure (by ref)"))
  (if (== OtherActor (`GameplayStatics.GetPlayerPawn` 0))
    ;[1 1 1] Add a process to add the unique key to inventory
    (`KismetSystemLibrary.PrintString` "Add a process to add the unique key to inventory")
    (`self.K2_DestroyActor`)))

(fn `UserConstructionScript`)