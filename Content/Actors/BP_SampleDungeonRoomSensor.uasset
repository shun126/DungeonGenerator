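; Sample dungeon room sensor whose OnInitialize event is empty, so it spawns nothing through its own graph.
; An unconnected example graph mirrors the SpawnActorInRoom parameter helper, which the author notes spawns automatically when parameters are set.
; That example runs on authority, scattering up to three area-scaled enemies in Hall and Hanare rooms using local random transforms.
; It also spawns Key or Unique Key items, though their spawn transforms are left unwired.
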(event `self.OnInitialize`
  (params (parts :type "EDungeonRoomParts Enum" :default "Any") (item :type "EDungeonRoomItem Enum" :default "Empty") (depthFromStart :type Byte) (depthFromStartRatio :type "Float (single-precision)")))

(fn `UserConstructionScript`)